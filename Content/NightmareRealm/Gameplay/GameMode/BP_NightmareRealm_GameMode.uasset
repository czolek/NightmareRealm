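; Game mode for NightmareRealm that runs a level where the wizard fights enemies to fill a pylon's energy and keep it from destruction.
; A looping timer tops up enemies at random spawners, picking types from a data table by level and chance.
; Damage and kill energy feed PlayerState, whose events drive death with resurrection countdown, level completion or game over.
; GetAttackTargetFor randomly splits attackers between player and pylon, capping player attackers.
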(event Custom|ControlEnemiesState
  ;[1 1 1] Verify how many enemies are in the level and spawn as many as needed to fill the quota
  (bind _maxreached (CallFunction|IsEnemyQuotaMet))
  (if (not _maxreached)
    (Utilities|FlowControl|DoOnce false
      (:Completed
        (CallFunction|SpawnEnemies)))))

(event Custom|SpawnEnemies
  ;[1 1 1] Spawn enemy
  (bind (_maxreached _stillmissingno) (CallFunction|IsEnemyQuotaMet))
  (if (not _maxreached)
    (for _index (range 1 _stillmissingno)
      (Utilities|FlowControl|Delay 0.5)
      (bind _enemytospawn (CallFunction|PickEnemytoSpawn))
      (Default|SpawnEnemy (.OutItem (Utilities|Array|Random (Variables|Internals|GetSpawners))) (.EnemyCharacterClass (Utilities|Struct|BreakS_EnemyStats _enemytospawn))))
    ;[1 1 1] Verify how many enemies are in the level and spawn as many as needed to fill the quota
    (Utilities|FlowControl|DoOnce false) ; enters at Reset
  ))

(event Custom|HandlePylonEnergyFilled
  (bind _fadeinoutduration (Utilities|GetClassDefaults "/Game/NightmareRealm/Misc/O_DataStorage.O_DataStorage_C"))
  ;[1 1 1] Pylon energy filled - level finished
  (Utilities|FlowControl|Sequence
    (:then_0
      (Variables|/Script/Engine.Actor|SetbCanBeDamaged (Variables|Internals|GetPylonRef) false) ; Stop Pylon from being damaged, so that we cannot loose when we've just won the level
    )
    (:then_1
      (Variables|/Script/Engine.Actor|SetbCanBeDamaged (Variables|Internals|GetPlayerCharacterRef) false) ; Same for the player
    )
    (:then_2
      (Default|Celebrate (Variables|Internals|GetPlayerCharacterRef))
      (Default|DisablePlayerControl (Variables|Internals|GetPlayerControllerRef)))
    (:then_3
      (CallFunction|StopEnemySpawning))
    (:then_4
      (Default|EnergyFull (Variables|Internals|GetPylonRef))
      (Utilities|FlowControl|Delay 3.0)
      (CallFunction|KillAllEnemies)
      (Utilities|FlowControl|Delay 1.0)
      (CameraFades|StartCameraFade :self (Game|GetPlayerCameraManager 0) :ToAlpha 1.0 :Duration _fadeinoutduration :bShouldFadeAudio true :bHoldWhenFinished true)
      (Utilities|FlowControl|Delay (+ _fadeinoutduration 1.0))
      (Class|BPIGameInstanceActions|NextLevel(Message) (Variables|Internals|GetGameInstance)))))

(event Custom|StopEnemySpawning
  ;[1 1 1] Stop enemy spawning and destroy all spawned enemies
  (Utilities|FlowControl|Sequence
    (:then_0
      (Utilities|Time|ClearandInvalidateTimerbyHandle (Variables|Internals|GetControlEnemiesStateTimer)))
    (:then_1
      (for _array_element (Variables|Internals|GetSpawners)
        (Variables|/Game/NightmareRealm/Actors/EnemySpawner/BP_EnemySpawner.BP_EnemySpawner_C|SetIsActive _array_element false)))))

(event Custom|KillAllEnemies
  (bind _spawnedenemies (Variables|Internals|GetSpawnedEnemies))
  ;[1 1 1] Stop enemy spawning and destroy all spawned enemies
  (while (Utilities|Array|IsValidIndex _spawnedenemies)
    (Default|Kill (Utilities|Array|Get(acopy) _spawnedenemies))))

(event Custom|DestroyAllEnemies
  ;[1 1 1] Stop enemy spawning and destroy all spawned enemies
  (for _array_element (Variables|Internals|GetSpawnedEnemies)
    (Actor|DestroyActor _array_element)))

(event Custom|PlayerIsDead
  ;[1 1 1] On Player's death
  (bind _resurrectioncountdown (CallFunction|CalculateResurrectionCountdownTime))
  (Default|RunResurrectionCountdown (Variables|Internals|GetHudRef) _resurrectioncountdown)
  (Default|Died (Variables|Internals|GetPlayerCharacterRef))
  (Default|DisablePlayerControl (Variables|Internals|GetPlayerControllerRef))
  (Class|BPIGameInstanceActions|PlayerDied(Message) (Game|GetGameInstance)))

(event Custom|EnemyCharacterSpawned
  (params (SpawnedEnemy :type BP%20Enemy%20Character%20Base%20Object%20Reference))
  ;[1 1 1] Enemy spawning is an async process, once finished add it to the array of spawned enemies and bid events
  (EventDispatchers|BindEventtoOnDeath SpawnedEnemy (EventDispatchers|CreateEvent :!event Custom|OnEnemyDeath))
  (Utilities|Array|Add (Variables|Internals|GetSpawnedEnemies) SpawnedEnemy))

(event Custom|HandlePlayerDamageReceived
  (params (Damage :type Float%20%28double-precision%29))
  ;[1 1 1] Handle Player damage
  (Default|PlayerDamageReveived (Variables|Internals|GetPlayerStateRef) Damage))

(event Custom|OnEnemyDeath
  (params (EnemyRef :type BP%20Enemy%20Character%20Base%20Object%20Reference))
  ;[1 1 1] OnEnemyDeath
  (bind _energygain (Default|GetEnergyGain EnemyRef))
  (Default|PylonEnergyGained (Variables|Internals|GetPlayerStateRef) _energygain)
  (Utilities|Array|RemoveItem (Variables|Internals|GetSpawnedEnemies) EnemyRef))

(event Custom|HandlePylonDestroyed
  ;[1 1 1] Game Over
  (Class|BPIGameInstanceActions|PylonDestroyed(Message) (Variables|Internals|GetGameInstance))
  (Utilities|FlowControl|Sequence
    (:then_0
      (Default|Destroyed (Variables|Internals|GetPylonRef)))
    (:then_1
      (CallFunction|StopEnemySpawning))
    (:then_2
      (CallFunction|DestroyAllEnemies))
    (:then_3
      (Actor|DestroyActor (Variables|Internals|GetPlayerCharacterRef)))))

(event Custom|HandleResurrectionCountdownFinished
  (bind _playercharacterref (Variables|Internals|GetPlayerCharacterRef))
  ;[1 1 1] Player's resurrection
  (Utilities|IsValid _playercharacterref
    (:Is%20Valid
      (Default|Resurrect _playercharacterref)
      (Default|CallOnPlayerResurrected))))

(event Custom|HandlePylonDamageReceived
  (params (Damage :type Float%20%28double-precision%29))
  ;[1 1 1] Handle Pylon damage
  (Default|PylonDamageReceived (Variables|Internals|GetPlayerStateRef) Damage))

(event EventPostLogin
  (params (NewPlayer :type Player%20Controller%20Object%20Reference))
  ;[1 1 1] HUD is initialised later than GameMode (it is also quite late in lifecycle), so bind to its custom event OnInitializationFinished, to show level info, once all is ready to play
  (Utilities|FlowControl|Delay 1.0)
  (bind _currentlevel (Class|BPIGameInstanceActions|GetCurrentLevel(Message) (Variables|Internals|GetGameInstance)))
  (Default|ShowLevelInfo (Variables|Internals|GetHudRef) _currentlevel))

(event EventBeginPlay
  ;[1 1 1] Initial setup
  (Utilities|FlowControl|Sequence
    (:then_0
      (Variables|Internals|SetGameInstance (Game|GetGameInstance)))
    (:then_1
      (bind _aspc_wizard_controller (Utilities|Casting|CastToPC_WizardController (Game|GetPlayerController 0)))
      (Variables|Internals|SetPlayerControllerRef _aspc_wizard_controller))
    (:then_2
      (bind _asbp_nightmare_realm_hud (Utilities|Casting|CastToBP_NightmareRealm_HUD (HUD|GetHUD (Game|GetPlayerController 0))))
      (Variables|Internals|SetHudRef _asbp_nightmare_realm_hud))
    (:then_3
      (bind _outactors (Actor|GetAllActorsOfClass "/Game/NightmareRealm/Actors/EnemySpawner/BP_EnemySpawner.BP_EnemySpawner_C"))
      (bind _output_get (Variables|Internals|SetSpawners _outactors))
      (for _array_element _output_get
        (EventDispatchers|BindEventtoOnEnemySpawned _array_element (EventDispatchers|CreateEvent :!event Custom|EnemyCharacterSpawned))))
    (:then_4
      (bind _returnvalue (Utilities|Time|SetTimerbyEvent (EventDispatchers|CreateEvent :!event Custom|ControlEnemiesState) (Variables|Internals|GetControlEnemiesStateTimerTick) true true))
      (Variables|Internals|SetControlEnemiesStateTimer _returnvalue))
    (:then_5
      (bind _levelstats (Class|BPIGameInstanceActions|GetLevelStats(Message) (Variables|Internals|GetGameInstance)))
      (Variables|Internals|SetLevel%20Stats _levelstats))
    (:then_6
      (bind _asbp_wizard (Utilities|Casting|CastToBP_Wizard (Game|GetPlayerCharacter 0)))
      (bind _output_get_2 (Variables|Internals|SetPlayerCharacterRef _asbp_wizard))
      (EventDispatchers|BindEventtoOnDamageReceived _output_get_2 (EventDispatchers|CreateEvent :!event Custom|HandlePlayerDamageReceived)))
    (:then_7
      (bind _returnvalue_2 (Actor|GetActorOfClass "/Game/NightmareRealm/Actors/Pylon/BP_Pylon.BP_Pylon_C"))
      (bind _output_get_3 (Variables|Internals|SetPylonRef _returnvalue_2))
      (EventDispatchers|BindEventtoOnDamageReceived _output_get_3 (EventDispatchers|CreateEvent :!event Custom|HandlePylonDamageReceived)))
    (:then_8
      (bind _asbp_nightmare_realm_player_state (Utilities|Casting|CastToBP_NightmareRealm_PlayerState (Game|GetPlayerState 0)))
      (bind _output_get_4 (Variables|Internals|SetPlayerStateRef _asbp_nightmare_realm_player_state))
      (EventDispatchers|BindEventtoOnPlayerHealthDepleted _output_get_4 (EventDispatchers|CreateEvent :!event Custom|PlayerIsDead))
      (EventDispatchers|BindEventtoOnPylonHealthDepleted _output_get_4 (EventDispatchers|CreateEvent :!event Custom|HandlePylonDestroyed))
      (EventDispatchers|BindEventtoOnPylonEnergyFilled _output_get_4 (EventDispatchers|CreateEvent :!event Custom|HandlePylonEnergyFilled)))
    (:then_9
      (bind _returnvalue_3 (Utilities|GetDataTableRow "/Game/NightmareRealm/DataTables/DT_PlayerStats.DT_PlayerStats" "Wizard")
        (:then
          (Variables|Internals|SetPlayerStats _returnvalue_3))))))

(fn ConstructionScript)

(fn GetEnemiesAttackingPlayer
  (for _array_element (Variables|Internals|GetSpawnedEnemies)
    (bind _currentattacktarget (Class|BPIAiControllerEvents|GetCurrentAttackTarget(Message) (AI|GetAIController _array_element) _array_element))
    (if (== _currentattacktarget (Variables|Internals|GetPlayerCharacterRef))
      (Utilities|Array|AddUnique (LocalVariables|GetEnemies) _array_element)))
  (return (LocalVariables|GetEnemies)))

(fn IsEnemyQuotaMet
  (bind _spawnedenemies (Variables|Internals|GetSpawnedEnemies))
  (bind _level_stats (Variables|Internals|GetLevel%20Stats))
  (bind _maxnoofconcurrentenemies (Utilities|Struct|BreakS_LevelStats _level_stats))
  (bind _returnvalue (Utilities|Array|Length _spawnedenemies))
  (bind _returnvalue_2 (- _maxnoofconcurrentenemies _returnvalue))
  (if (> _returnvalue_2 0)
    (return false _returnvalue_2)
    (else
      (return true 0))))

(fn PickEnemytoSpawn
  (bind _enemies (|GetEnemiesDataTableRows)
    (:Completed
      (bind _enemiesmatchingcurrentlevel (|FilterEnemiesForCurrentLevel _enemies)
        (:Completed
          (bind _spawncandidate (|GetRandomEnemyToSpawn _enemiesmatchingcurrentlevel (Math|Random|RandomFloat))
            (:Completed
              (Development|PrintString (Utilities|String|Append "Spawning: " (Utilities|ToString(SoftClassReference) (.EnemyCharacterClass (Utilities|Struct|BreakS_EnemyStats _spawncandidate)))) false false)
              (return _spawncandidate))))))))

(fn CalculateResurrectionCountdownTime
  (bind _playerstats (Variables|Internals|GetPlayerStats))
  (bind (_basehealth _resurrectionbasecountdown _consecutivedeathresurrectioncountdownincrementby) (Utilities|Struct|BreakS_PlayerStats _playerstats))
  (bind _deathcount (Class|BPIGameInstanceActions|GetPlayerDeathCount(Message) (Game|GetGameInstance)))
  (return (+ (Math|Float|Round (* _deathcount _consecutivedeathresurrectioncountdownincrementby)) _resurrectionbasecountdown)))

(fn GetAttackTargetfor
  (params (Attacker :type Actor%20Object%20Reference))
  (bind _alive (Default|IsPlayerAlive (Variables|Internals|GetPlayerStateRef)))
  (if (and _alive (Math|Random|RandomBool))
    (bind _enemiesattackingplayer (CallFunction|GetEnemiesAttackingPlayer))
    (if (Utilities|Array|ContainsItem _enemiesattackingplayer Attacker)
      (return (Variables|Internals|GetPlayerCharacterRef)) ; If Attacker already attacks alive player, keep attacking
      (elif (< (Utilities|Array|Length _enemiesattackingplayer) (.MaxNoOfMeleePlayerAttackers (Utilities|Struct|BreakS_LevelStats (Variables|Internals|GetLevel%20Stats))))
        (return (Variables|Internals|GetPlayerCharacterRef)) ; If Attacker does not yet attack alive player and amount of player attackers is not maxed out then attack the player
        (else
          (return (Variables|Internals|GetPylonRef)) ; If Attacker does not yet attack alive player, but amount of player attackers is maxed out then attack the pylon
        )))
    (else
      (return (Variables|Internals|GetPylonRef)) ; If player is dead, attack the pylon, no questions asked
    )))