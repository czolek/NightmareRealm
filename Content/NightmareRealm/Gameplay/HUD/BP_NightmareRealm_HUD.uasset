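; Nightmare Realm HUD that shows player and pylon status, the level number and resurrection countdown, and handles the game-over screen.
; On BeginPlay it binds to GameMode and PlayerState events, seeds the main widget from GameInstance stats and creates hidden popup widgets.
; Event handlers push health and energy changes to the widget and report countdown completion to the GameMode.
; Pylon depletion triggers game over with UI mode and camera fade, while full energy just hides the HUD.
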(event Custom|HandlePlayerHealthReduced
  (params (CurrentHealth :type Float%20%28double-precision%29))
  ;[1 1 1] Player event handlers
  (Default|UpdatePlayerHealth (Variables|Internals|GetGameHudWidgetRef) CurrentHealth))

(event Custom|HandlePylonHealthReduced
  (params (CurrentHealth :type Float%20%28double-precision%29))
  ;[1 1 1] Pylon event handlers
  (Default|UpdatePylonHealth (Variables|Internals|GetGameHudWidgetRef) CurrentHealth))

(event Custom|ShowLevelInfo
  (params (LevelNo :type Integer))
  ;[1 1 1] Show level no widget
  (Widget|SetVisibility (Variables|Internals|GetLevelNoInfoWidget) "Visible")
  (UserInterface|Viewport|AddtoViewport (Variables|Internals|GetLevelNoInfoWidget) 0)
  (Default|DisplayLevelNo (Variables|Internals|GetLevelNoInfoWidget) LevelNo)
  (Audio|PlaySound2D "/Game/NightmareRealm/Gameplay/Menus/LevelStart/PossessPlayer_Cue.PossessPlayer_Cue" 1.0 1.0 0.0 0 0)
  (Utilities|FlowControl|Delay 2.0)
  (CallFunction|HideLevelInfo))

(event Custom|HandlePylonEnergyFilled
  ;[1 1 1] Pylon event handlers
  (Default|Hide (Variables|Internals|GetGameHudWidgetRef)))

(event Custom|HandlePylonHealthDepleted
  ;[1 1 1] Pylon event handlers
  (Utilities|FlowControl|Sequence
    (:then_0
      (Default|Hide (Variables|Internals|GetGameHudWidgetRef)))
    (:then_1
      (bind _returnvalue (UserInterface|CreateWidget "/Game/NightmareRealm/Gameplay/Menus/GameOverScreen/UI_GameOverScreen.UI_GameOverScreen_C" (Game|GetPlayerController 0)))
      (UserInterface|Viewport|AddtoViewport _returnvalue 0)
      (Class|BPIPlayerControllerActions|DisablePlayerControl(Message) (Game|GetPlayerController 0))
      (Class|BPIPlayerControllerActions|EnableUIMode(Message) (Game|GetPlayerController 0))
      (Audio|PlaySound2D "/Game/NightmareRealm/Gameplay/Menus/GameOverScreen/SW_Bell_Cue.SW_Bell_Cue" 1.0 1.0 0.0 0 0))
    (:then_2
      (CameraFades|StartCameraFade :self (Variables|/Script/Engine.PlayerController|GetPlayerCameraManager (Game|GetPlayerController 0)) :ToAlpha 1.0 :Duration (Variables|Editable|GetCameraFadeDuration) :bShouldFadeAudio true :bHoldWhenFinished true))))

(event Custom|HandleOnPylonEnergyIncreased
  (params (CurrentEnergy :type Float%20%28double-precision%29))
  ;[1 1 1] Pylon event handlers
  (Default|UpdatePylonEnergy (Variables|Internals|GetGameHudWidgetRef) CurrentEnergy))

(event Custom|HandlePlayerResurrected
  ;[1 1 1] Player event handlers
  (bind _health (Class|BPISkillSupplier|GetPlayerHealthStats(Message) (Game|GetGameInstance)))
  (Default|UpdatePlayerHealth (Variables|Internals|GetGameHudWidgetRef) _health))

(event Custom|HandleResurrectCountdownFinished
  ;[1 1 1] Player event handlers
  (Widget|RemovefromParent (Variables|Internals|GetResurrectCountdownWidget))
  (Widget|SetVisibility (Variables|Internals|GetResurrectCountdownWidget) "Hidden")
  (bind _asbp_nightmare_realm_game_mode (Utilities|Casting|CastToBP_NightmareRealm_GameMode (Game|GetGameMode)))
  (Default|HandleResurrectionCountdownFinished _asbp_nightmare_realm_game_mode))

(event Custom|RunResurrectionCountdown
  (params (Time :type Integer))
  ;[1 1 1] Player event handlers
  (Widget|SetVisibility (Variables|Internals|GetResurrectCountdownWidget) "Visible")
  (UserInterface|Viewport|AddtoViewport (Variables|Internals|GetResurrectCountdownWidget) 0)
  (Default|RunCountdown (Variables|Internals|GetResurrectCountdownWidget) Time))

(event Custom|HideLevelInfo
  ;[1 1 1] Show level no widget
  (Widget|RemovefromParent (Variables|Internals|GetLevelNoInfoWidget))
  (Widget|SetVisibility (Variables|Internals|GetLevelNoInfoWidget) "Hidden"))

(event EventBeginPlay
  (bind _returnvalue (Game|GetGameInstance))
  ;[1 1 1] Setup
  (Utilities|FlowControl|Sequence
    (:then_0
      (bind _asbp_nightmare_realm_game_mode (Utilities|Casting|CastToBP_NightmareRealm_GameMode (Game|GetGameMode)))
      (EventDispatchers|BindEventtoOnPlayerResurrected _asbp_nightmare_realm_game_mode (EventDispatchers|CreateEvent :!event Custom|HandlePlayerResurrected)))
    (:then_1
      (bind _asbp_nightmare_realm_player_state (Utilities|Casting|CastToBP_NightmareRealm_PlayerState (Game|GetPlayerState 0)))
      (bind _output_get (Variables|Internals|SetPlayerStateRef _asbp_nightmare_realm_player_state))
      (EventDispatchers|BindEventtoOnPlayerHealthReduced _output_get (EventDispatchers|CreateEvent :!event Custom|HandlePlayerHealthReduced))
      (EventDispatchers|BindEventtoOnPylonHealthReduced _output_get (EventDispatchers|CreateEvent :!event Custom|HandlePylonHealthReduced))
      (EventDispatchers|BindEventtoOnPylonHealthDepleted _output_get (EventDispatchers|CreateEvent :!event Custom|HandlePylonHealthDepleted))
      (EventDispatchers|BindEventtoOnPylonEnergyIncreased _output_get (EventDispatchers|CreateEvent :!event Custom|HandleOnPylonEnergyIncreased))
      (EventDispatchers|BindEventtoOnPylonEnergyFilled _output_get (EventDispatchers|CreateEvent :!event Custom|HandlePylonEnergyFilled)))
    (:then_2
      (bind _asbp_hud_widget (Utilities|Casting|CastToBP_HUD_Widget (UserInterface|GetWidget (Variables|Default|GetHud))))
      (bind _output_get_2 (Variables|Internals|SetGameHudWidgetRef _asbp_hud_widget))
      (UserInterface|Viewport|AddtoViewport _output_get_2 0)
      (Utilities|FlowControl|Sequence
        (:then_0
          (bind _health (Class|BPISkillSupplier|GetPlayerHealthStats(Message) _returnvalue))
          (Default|SetInitialPlayerHealth (Variables|Internals|GetGameHudWidgetRef) _health))
        (:then_1
          (bind _health_2 (Class|BPISkillSupplier|GetPylonHealthStats(Message) _returnvalue))
          (Default|SetInitialPylonHealth (Variables|Internals|GetGameHudWidgetRef) _health_2))
        (:then_2
          (bind _energy (Class|BPISkillSupplier|GetPylonEnergyStats(Message) _returnvalue))
          (Default|SetInitialPylonEnergyCapacity (Variables|Internals|GetGameHudWidgetRef) _energy))))
    (:then_3
      (bind _returnvalue_2 (UserInterface|CreateWidget "/Game/NightmareRealm/Gameplay/Menus/ResurrectionCountdown/UI_ResurrectCountdown.UI_ResurrectCountdown_C"))
      (bind _output_get_3 (Variables|Internals|SetResurrectCountdownWidget _returnvalue_2))
      (Widget|SetVisibility _output_get_3 "Hidden"))
    (:then_4
      (bind _returnvalue_3 (UserInterface|CreateWidget "/Game/NightmareRealm/Gameplay/Menus/LevelStart/UI_LevelStart.UI_LevelStart_C"))
      (bind _output_get_4 (Variables|Internals|SetLevelNoInfoWidget _returnvalue_3))
      (Widget|SetVisibility _output_get_4 "Hidden"))
    (:then_5
      (Class|BPISkillSupplier|GetEnabledSkillsInfo(Message) (Game|GetGameInstance)))))

(fn ConstructionScript)