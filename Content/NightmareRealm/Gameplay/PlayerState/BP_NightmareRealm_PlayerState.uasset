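; Player state for Nightmare Realm that tracks player health, pylon health and pylon energy.
; On BeginPlay it creates a refillable container component for each, sized from game instance stats.
; Incoming damage and energy events adjust the containers, whose change, empty and full notifications are re-broadcast through dispatchers, intended for the HUD.
; Player health replenishes when the game mode signals resurrection, and helper functions report whether player and pylon are alive.
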(event Custom|HandlePlayerHealthReduced
  (params (CurrentHealth :type Float%20%28double-precision%29))
  ;[1 1 1] Player
  ;;[1 1 1] When Player Health component notifies about health reduction, send event to HUD
  (Default|CallOnPlayerHealthReduced CurrentHealth))

(event Custom|HandlePlayerHealthDepleted
  ;[1 1 1] Player
  ;;[1 1 1] Player health depleted
  (Default|CallOnPlayerHealthDepleted))

(event Custom|HandlePylonHealthReduced
  (params (CurrentHealth :type Float%20%28double-precision%29))
  ;[1 1 1] Pylon
  ;;[1 1 1] When Pylon Health component notifies about health reduction, send event to HUD
  (Default|CallOnPylonHealthReduced CurrentHealth))

(event Custom|HandlePylonHealthDepleted
  ;[1 1 1] Pylon
  ;;[1 1 1] Pylon health depleted
  (Default|CallOnPylonHealthDepleted))

(event Custom|HandlePlayerResurrected
  ;[1 1 1] Reset default player health after resurrection
  (Default|Replenish (Variables|Default|GetPlayerHealth)))

(event Custom|HandlePylonEnergyIncreased
  (params (CurrentFillLevel :type Float%20%28double-precision%29))
  ;[1 1 1] Pylon
  ;;[1 1 1] When Pylon Energy component notifies about energy increase, send event to HUD
  (Default|CallOnPylonEnergyIncreased CurrentFillLevel))

(event Custom|HandlePylonEnergyFilled
  ;[1 1 1] Pylon
  ;;[1 1 1] Pylon energy filled
  (Default|CallOnPylonEnergyFilled)
  (Development|PrintString "Pylon ENERGY FULL"))

(event Custom|PlayerDamageReveived
  (params (Damage :type Float%20%28double-precision%29))
  ;[1 1 1] Apply player damage to health component
  (Default|DecreaseFillLevel (Variables|Default|GetPlayerHealth) Damage))

(event Custom|PylonDamageReceived
  (params (Damage :type Float%20%28double-precision%29))
  ;[1 1 1] Apply pylon damage to health component
  (Default|DecreaseFillLevel (Variables|Default|GetPylonHealth) Damage))

(event Custom|PylonEnergyGained
  (params (Amount :type Float%20%28double-precision%29))
  ;[1 1 1] Increase pylon energy level
  (Default|IncreaseFillLevel (Variables|Default|GetPylonEnergy) Amount))

(event EventBeginPlay
  ;[1 1 1] Setup health components
  (Utilities|FlowControl|Sequence
    (:then_0
      (bind _asbp_nightmare_realm_game_mode (Utilities|Casting|CastToBP_NightmareRealm_GameMode (Game|GetGameMode)))
      (EventDispatchers|BindEventtoOnPlayerResurrected _asbp_nightmare_realm_game_mode (EventDispatchers|CreateEvent :!event Custom|HandlePlayerResurrected)))
    (:then_1
      (bind _basehealth (CallFunction|GetDefaultPlayerHealth))
      (bind _returnvalue (Game|AddComponentbyClass :Class "/Game/NightmareRealm/Components/Health/AC_RefillableContainer.AC_RefillableContainer_C" :InitialFillLevel _basehealth :HasFillLevelBar false :MaxCapacity _basehealth))
      (bind _output_get (Variables|Default|SetPlayerHealth _returnvalue))
      (EventDispatchers|AssignOnFillLevelDecreased _output_get (EventDispatchers|CreateEvent :!event Custom|HandlePlayerHealthReduced))
      (EventDispatchers|BindEventtoOnEmptied (Variables|Default|GetPlayerHealth) (EventDispatchers|CreateEvent :!event Custom|HandlePlayerHealthDepleted)))
    (:then_2
      (bind _basehealth_2 (CallFunction|GetDefaultPylonHealth))
      (bind _returnvalue_2 (AddComponent|AddACRefillableContainer :InitialFillLevel _basehealth_2 :HasFillLevelBar false :MaxCapacity _basehealth_2))
      (bind _output_get_2 (Variables|Default|SetPylonHealth _returnvalue_2))
      (EventDispatchers|BindEventtoOnFillLevelDecreased _output_get_2 (EventDispatchers|CreateEvent :!event Custom|HandlePylonHealthReduced))
      (EventDispatchers|BindEventtoOnEmptied (Variables|Default|GetPylonHealth) (EventDispatchers|CreateEvent :!event Custom|HandlePylonHealthDepleted)))
    (:then_3
      (bind _baseenergycapacity (CallFunction|GetDefaultPylonEnergyCapacity))
      (bind _returnvalue_3 (AddComponent|AddACRefillableContainer :InitialFillLevel (Variables|Internals|GetInitialPylonEnergyLevel) :MaxCapacity _baseenergycapacity))
      (bind _output_get_3 (Variables|Default|SetPylonEnergy _returnvalue_3))
      (EventDispatchers|BindEventtoOnFillLevelIncreased _output_get_3 (EventDispatchers|CreateEvent :!event Custom|HandlePylonEnergyIncreased))
      (EventDispatchers|BindEventtoOnFilled (Variables|Default|GetPylonEnergy) (EventDispatchers|CreateEvent :!event Custom|HandlePylonEnergyFilled)))))

(fn ConstructionScript)

(fn GetDefaultPylonEnergyCapacity
  (bind _energy (Class|BPISkillSupplier|GetPylonEnergyStats(Message) (Game|GetGameInstance)))
  (Development|PrintString (Utilities|String|Append "Pylon's energy: " (Utilities|String|ToString(Float) _energy)))
  (return _energy))

(fn GetDefaultPylonHealth
  (bind _health (Class|BPISkillSupplier|GetPylonHealthStats(Message) (Game|GetGameInstance)))
  (Development|PrintString (Utilities|String|Append "Pylon's health: " (Utilities|String|ToString(Float) _health)))
  (return _health))

(fn GetDefaultPlayerHealth
  (bind _health (Class|BPISkillSupplier|GetPlayerHealthStats(Message) (Game|GetGameInstance)))
  (Development|PrintString (Utilities|String|Append "Player's health: " (Utilities|String|ToString(Float) _health)))
  (return _health))

(fn IsPylonAlive
  (return (Default|IsNotEmpty (Variables|Default|GetPylonHealth))))

(fn IsPlayerAlive
  (return (Default|IsNotEmpty (Variables|Default|GetPlayerHealth))))