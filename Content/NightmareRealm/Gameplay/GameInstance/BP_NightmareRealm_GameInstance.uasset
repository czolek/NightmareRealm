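; Game instance for Nightmare Realm that holds run progress (level, death count, enabled skills) and drives new game, continue, level-up and level loading through a loading screen.
; Level-ups merge a data table row into the enabled skills, show a skill-card widget, then save and restart the level.
; Progress persists through async save slots, deleted when the pylon is destroyed.
; Getters combine data tables with level and skills to supply player, weapon and pylon stats.
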(event Custom|LoadMainLevel
  ;[1 1 1] Show loading screen
  (Class|BPIStreamingLevelActions|UnloadLevel(Message) (Class|GameplayStatics|GetStreamingLevel (Variables|Levels|GetL_MainMenu)))
  (Game|LoadStreamLevel(byName) (Variables|Levels|GetL_LoadingScreen) true)
  (Class|BPIStreamingLevelActions|RunLevel(Message) (Class|GameplayStatics|GetStreamingLevel (Variables|Levels|GetL_LoadingScreen)))
  (Utilities|FlowControl|Delay 1.0)
  ;[1 1 1] Load actual game level
  (Game|LoadStreamLevel(byName) (Variables|Levels|GetL_NightmareRealm) false)
  (Class|BPIStreamingLevelActions|UnloadLevel(Message) (Class|GameplayStatics|GetStreamingLevel (Variables|Levels|GetL_LoadingScreen)))
  (Game|OpenLevel(byObjectReference) "/Game/NightmareRealm/Levels/L_NightmareRealm.L_NightmareRealm"))

(event Custom|LevelUpContinue
  ;[1 1 1] New level
  (Widget|RemovefromParent (Variables|Internals|GetLevelUpWidget))
  (Class|BPIPlayerControllerActions|EnableGameMode(Message) (Game|GetPlayerController 0))
  (CallFunction|SaveProgress)
  (Development|ExecuteConsoleCommand "RestartLevel" 0)
  (CameraFades|StartCameraFade :self (Game|GetPlayerCameraManager 0) :FromAlpha 1.0 :Duration 1.0 :bShouldFadeAudio true :bHoldWhenFinished true))

(event EventNextLevel
  ;[1 1 1] New level
  (Math|Integer|IncrementInt (Variables|Internals|GetLevel)
    (:%20%20
      (CallFunction|PrepareLevelUp)
      (Class|BPIPlayerControllerActions|EnableUIMode(Message) (Game|GetPlayerController 0))
      (UserInterface|Viewport|AddtoViewport (Variables|Internals|GetLevelUpWidget) 0)
      (Default|FlipSkillCard (Variables|Internals|GetLevelUpWidget)))))

(event EventStartNewGame
  ;[1 1 1] Delete old save game (if exists) and create a new one
  (Utilities|FlowControl|Sequence
    (:then_0
      (Variables|Internals|SetLevel 1)
      (Variables|Internals|SetPlayerDeathCount 0)
      (Variables|Internals|SetEnabledSkills (Variables|Internals|GetDefaultSkills)))
    (:then_1
      (bind _exists (CallFunction|DoesProgressSaveExist))
      (if _exists
        (SaveGame|DeleteGameinSlot (Variables|SaveGame|GetProgressSaveGameSlot)))
      (bind _returnvalue (SaveGame|CreateSaveGameObject "/Game/NightmareRealm/Gameplay/SaveGame/BP_ProgressSaveGame.BP_ProgressSaveGame_C"))
      (Variables|SaveGame|SetProgressSaveGameRef _returnvalue)
      (CallFunction|SaveProgress)
      (CallFunction|LoadMainLevel))))

(event EventSaveProgress
  ;[1 1 1] Save game progress
  (bind _exists (CallFunction|DoesProgressSaveExist))
  (if _exists
    (Variables|SaveGame|GetProgressSaveGameRef
      (:then
        _)
      (:else
        (bind _returnvalue (SaveGame|CreateSaveGameObject "/Game/NightmareRealm/Gameplay/SaveGame/BP_ProgressSaveGame.BP_ProgressSaveGame_C" :!label _label))
        (Variables|SaveGame|SetProgressSaveGameRef _returnvalue)))
    (else
      (goto _label)))
  (Variables|/Game/NightmareRealm/Gameplay/SaveGame/BP_ProgressSaveGame.BP_ProgressSaveGame_C|SetLevelNo (Variables|SaveGame|GetProgressSaveGameRef) (Variables|Internals|GetLevel))
  (Variables|/Game/NightmareRealm/Gameplay/SaveGame/BP_ProgressSaveGame.BP_ProgressSaveGame_C|SetPlayerDeathCount (Variables|SaveGame|GetProgressSaveGameRef) (Variables|Internals|GetPlayerDeathCount))
  (Variables|/Game/NightmareRealm/Gameplay/SaveGame/BP_ProgressSaveGame.BP_ProgressSaveGame_C|SetEnabledSkills (Variables|SaveGame|GetProgressSaveGameRef) (Variables|Internals|GetEnabledSkills))
  (|AsyncSaveGametoSlot (Variables|SaveGame|GetProgressSaveGameRef) (Variables|SaveGame|GetProgressSaveGameSlot)))

(event EventPlayerDied
  ;[1 1 1] Player death
  (Math|Integer|IncrementInt (Variables|Internals|GetPlayerDeathCount)))

(event EventInit
  ;[1 1 1] Init
  (bind _returnvalue (UserInterface|CreateWidget "/Game/NightmareRealm/Gameplay/Menus/LevelUp/UI_LevelUp.UI_LevelUp_C"))
  (bind _output_get (Variables|Internals|SetLevelUpWidget _returnvalue))
  (EventDispatchers|BindEventtoOnContinueButtonClicked _output_get (EventDispatchers|CreateEvent :!event Custom|LevelUpContinue)))

(event EventPylonDestroyed
  ;[1 1 1] Game over, delete progress save game
  (SaveGame|DeleteGameinSlot (Variables|SaveGame|GetProgressSaveGameSlot)))

(event EventContinueGame
  ;[1 1 1] Load game and start gameplay
  (bind _savegame (|AsyncLoadGamefromSlot (Variables|SaveGame|GetProgressSaveGameSlot))
    (:Completed
      (bind _asbp_progress_save_game (Utilities|Casting|CastToBP_ProgressSaveGame _savegame))
      (Variables|SaveGame|SetProgressSaveGameRef _asbp_progress_save_game)
      (Variables|Internals|SetLevel (Variables|/Game/NightmareRealm/Gameplay/SaveGame/BP_ProgressSaveGame.BP_ProgressSaveGame_C|GetLevelNo (Variables|SaveGame|GetProgressSaveGameRef)))
      (Variables|Internals|SetPlayerDeathCount (Variables|/Game/NightmareRealm/Gameplay/SaveGame/BP_ProgressSaveGame.BP_ProgressSaveGame_C|GetPlayerDeathCount (Variables|SaveGame|GetProgressSaveGameRef)))
      (Variables|Internals|SetEnabledSkills (Variables|/Game/NightmareRealm/Gameplay/SaveGame/BP_ProgressSaveGame.BP_ProgressSaveGame_C|GetEnabledSkills (Variables|SaveGame|GetProgressSaveGameRef)))
      (CallFunction|LoadMainLevel))))

(event EventLoadMainMenu
  ;[1 1 1] Used on game over to get back to main menu
  (Game|OpenLevel(byObjectReference) "/Game/NightmareRealm/Levels/L_PersistentLevel.L_PersistentLevel"))

(fn PrepareLevelUp
  (bind _statsforcurrentlevel (LocalVariables|GetStatsForCurrentLevel))
  (bind (_skillsmodifier _name _icon) (Utilities|Struct|BreakS_LevelUpDefinition _statsforcurrentlevel))
  (bind (_firebalenabled _explosivefireballenabled _inceneratingfireballenabled _lifemultiplier _spellcastspeedmultiplier _meleeattackspeedmultiplier _doublestaffswingenabled) (Utilities|Struct|BreakS_SkillsModifier _skillsmodifier))
  (|SetLevelUpStatsForCurrentLevel)
  (Variables|/Game/NightmareRealm/Gameplay/Menus/LevelUp/UI_LevelUp.UI_LevelUp_C|SetSkillName (Variables|Internals|GetLevelUpWidget) _name)
  (Variables|/Game/NightmareRealm/Gameplay/Menus/LevelUp/UI_LevelUp.UI_LevelUp_C|SetSkillImageTexture (Variables|Internals|GetLevelUpWidget) _icon)
  (Variables|Internals|SetEnabledSkills (Utilities|Struct|MakeS_SkillsModifier (or _firebalenabled (.FirebalEnabled (Utilities|Struct|BreakS_SkillsModifier (Variables|Internals|GetEnabledSkills)))) (or _explosivefireballenabled (.ExplosiveFireballEnabled (Utilities|Struct|BreakS_SkillsModifier (Variables|Internals|GetEnabledSkills)))) (or _inceneratingfireballenabled (.InceneratingFireballEnabled (Utilities|Struct|BreakS_SkillsModifier (Variables|Internals|GetEnabledSkills)))) (* _lifemultiplier (.LifeMultiplier (Utilities|Struct|BreakS_SkillsModifier (Variables|Internals|GetEnabledSkills)))) (* _spellcastspeedmultiplier (.SpellCastSpeedMultiplier (Utilities|Struct|BreakS_SkillsModifier (Variables|Internals|GetEnabledSkills)))) (* _meleeattackspeedmultiplier (.MeleeAttackSpeedMultiplier (Utilities|Struct|BreakS_SkillsModifier (Variables|Internals|GetEnabledSkills)))) (or _doublestaffswingenabled (.DoubleStaffSwingEnabled (Utilities|Struct|BreakS_SkillsModifier (Variables|Internals|GetEnabledSkills)))))))

(fn DoesProgressSaveExist
  (bind _returnvalue (SaveGame|DoesSaveGameExist (Variables|SaveGame|GetProgressSaveGameSlot)))
  (return _returnvalue))

(fn GetCurrentLevel
  (return (Variables|Internals|GetLevel)))

(fn GetEnabledSkillsInfo
  (bind _outrownames (DataTable|GetDataTableRowNames "/Game/NightmareRealm/DataTables/DT_LevelUpStats.DT_LevelUpStats"))
  (bind (_array_element _array_index) (Utilities|Array|ForEachLoopwithBreak _outrownames :!label _label)
    (:LoopBody
      (if (<= (+ _array_index 2) (Variables|Internals|GetLevel))
        (bind _returnvalue (Utilities|GetDataTableRow "/Game/NightmareRealm/DataTables/DT_LevelUpStats.DT_LevelUpStats" _array_element)
          (:then
            (Utilities|Array|Add (LocalVariables|GetSkillIcons) (.Icon (Utilities|Struct|BreakS_LevelUpDefinition _returnvalue)))))
        (else
          (goto _label Break))))
    (:Completed
      (return (LocalVariables|GetSkillIcons)))))

(fn GetFireballSkillStats
  (bind _enabledskills (Variables|Internals|GetEnabledSkills))
  (bind (_firebalenabled _explosivefireballenabled _inceneratingfireballenabled _lifemultiplier _spellcastspeedmultiplier) (Utilities|Struct|BreakS_SkillsModifier _enabledskills))
  (bind _returnvalue (Utilities|GetDataTableRow "/Game/NightmareRealm/DataTables/DT_Weapons.DT_Weapons" "FireBall")
    (:then
      (for _array_element (.Effects (Utilities|Struct|BreakS_WeaponStats _returnvalue))
        (switch Utilities|FlowControl|Switch|SwitchonE_DamageType (.Type (Utilities|Struct|BreakS_WeaponEffects _array_element))
          (:NewEnumerator5
            (LocalVariables|SetBurnDamage (.Damage (Utilities|Struct|BreakS_WeaponEffects _array_element)))
            (LocalVariables|SetBurnRadius (.Radius (Utilities|Struct|BreakS_WeaponEffects _array_element)))
            (LocalVariables|SetDotTick (.DoTTickFrequency (Utilities|Struct|BreakS_WeaponEffects _array_element))))
          (:NewEnumerator6
            (LocalVariables|SetExplosiveDamage (.Damage (Utilities|Struct|BreakS_WeaponEffects _array_element)))
            (LocalVariables|SetExplosiveRadius (.Radius (Utilities|Struct|BreakS_WeaponEffects _array_element))))))
      (return (Utilities|Struct|MakeS_FireballSkillStats _firebalenabled _explosivefireballenabled _inceneratingfireballenabled (* _spellcastspeedmultiplier (.AttackSpeed (Utilities|Struct|BreakS_WeaponStats _returnvalue))) (.BaseDamage (Utilities|Struct|BreakS_WeaponStats _returnvalue)) (LocalVariables|GetExplosiveDamage) (LocalVariables|GetExplosiveRadius) (LocalVariables|GetBurnDamage) (LocalVariables|GetBurnRadius) (LocalVariables|GetDotTick))))))

(fn GetLevelStats
  (bind _outrownames (DataTable|GetDataTableRowNames "/Game/NightmareRealm/DataTables/DT_LevelStats.DT_LevelStats"))
  (LocalVariables|SetDataRowNames _outrownames)
  (if (> (Utilities|Array|FindItem (LocalVariables|GetDataRowNames) (Utilities|String|StringToName (Utilities|String|ToString(Integer) (Variables|Internals|GetLevel)))) -1)
    (bind _returnvalue (Utilities|GetDataTableRow "/Game/NightmareRealm/DataTables/DT_LevelStats.DT_LevelStats" (Utilities|Array|Get(acopy) (LocalVariables|GetDataRowNames) (Utilities|Array|FindItem (LocalVariables|GetDataRowNames) (Utilities|String|StringToName (Utilities|String|ToString(Integer) (Variables|Internals|GetLevel))))))
      (:then
        (return _returnvalue)))
    (else
      (bind _returnvalue_2 (Utilities|GetDataTableRow "/Game/NightmareRealm/DataTables/DT_LevelStats.DT_LevelStats" (Utilities|Array|Get(acopy) (LocalVariables|GetDataRowNames) (Utilities|Array|LastIndex (LocalVariables|GetDataRowNames))))
        (:then
          (return _returnvalue_2))))))

(fn GetMagicStaffSkillStats
  (bind _enabledskills (Variables|Internals|GetEnabledSkills))
  (bind (_firebalenabled _explosivefireballenabled _inceneratingfireballenabled _lifemultiplier _spellcastspeedmultiplier _meleeattackspeedmultiplier _doublestaffswingenabled) (Utilities|Struct|BreakS_SkillsModifier _enabledskills))
  (bind _returnvalue (Utilities|GetDataTableRow "/Game/NightmareRealm/DataTables/DT_Weapons.DT_Weapons" "MageStaff")
    (:then
      (if _doublestaffswingenabled
        (return (.BaseDamage (Utilities|Struct|BreakS_WeaponStats _returnvalue)) (* _meleeattackspeedmultiplier (.AttackSpeed (Utilities|Struct|BreakS_WeaponStats _returnvalue))) "/Game/NightmareRealm/Actors/BattleWizard/Animations/AM_StaffAttack_Level2.AM_StaffAttack_Level2")
        (else
          (return (.BaseDamage (Utilities|Struct|BreakS_WeaponStats _returnvalue)) (* _meleeattackspeedmultiplier (.AttackSpeed (Utilities|Struct|BreakS_WeaponStats _returnvalue))) "/Game/NightmareRealm/Actors/BattleWizard/Animations/AM_StaffAttack_Basic.AM_StaffAttack_Basic"))))))

(fn GetPlayerDeathCount
  (return (Variables|Internals|GetPlayerDeathCount)))

(fn GetPlayerHealthStats
  (bind _returnvalue (Utilities|GetDataTableRow "/Game/NightmareRealm/DataTables/DT_PlayerStats.DT_PlayerStats" "Wizard")
    (:then
      (return (* (.BaseHealth (Utilities|Struct|BreakS_PlayerStats _returnvalue)) (.LifeMultiplier (Utilities|Struct|BreakS_SkillsModifier (Variables|Internals|GetEnabledSkills))))))))

(fn GetPylonEnergyStats
  (bind _returnvalue (Utilities|GetDataTableRow "/Game/NightmareRealm/DataTables/DT_PylonStats.DT_PylonStats" "Pylon")
    (:then
      (return (* (.BaseEnergyCapacity (Utilities|Struct|BreakS_PylonStats _returnvalue)) (Math|Float|Power (.EnergyIncreasePerLevel (Utilities|Struct|BreakS_PylonStats _returnvalue)) (Math|Conversions|ToFloat(Integer) (- (Variables|Internals|GetLevel) 1))))))))

(fn GetPylonHealthStats
  (bind _returnvalue (Utilities|GetDataTableRow "/Game/NightmareRealm/DataTables/DT_PylonStats.DT_PylonStats" "Pylon")
    (:then
      (return (.BaseHealth (Utilities|Struct|BreakS_PylonStats _returnvalue))))))