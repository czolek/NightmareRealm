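; Scene component that creates a fire hazard, with an attached particle effect and periodic radial damage around its location.
; StartFire runs once, spawning the emitter and starting a looping timer for damage ticks.
; Each tick applies radial damage that skips ignored actors and uses the Pawn channel as its damage prevention channel.
; EndPlay clears the timer and destroys the particle component.
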(event Custom|StartFire
  ;[1 1 1] Start a fire - spawn particle component and start ticking damage
  (Utilities|FlowControl|DoOnce false
    (:Completed
      (|SpawnFire)
      (bind _returnvalue (Utilities|Time|SetTimerbyEvent (EventDispatchers|CreateEvent :!event Custom|TickFireDamage) (Variables|Editable|GetFireTimerTick) true true))
      (Variables|Default|SetDamageTimerHandle _returnvalue))))

(event Custom|TickFireDamage
  ;[1 1 1] Apply damage to any pawn in a radius
  (Game|Damage|ApplyRadialDamage (Variables|Editable|GetFireDamagePerTick) (Transformation|GetWorldLocation) (Variables|Editable|GetFireRadius) 0 (Variables|Editable|GetIgnore%20Actors) 0 0 false "ECC_Pawn"))

(event EventEndPlay
  (params (EndPlayReason :type EEndPlayReason%20Enum :default "Destroyed"))
  (bind _fire (Variables|Default|GetFire))
  ;[1 1 1] Deactivate and destroy spawned fire particle component
  (Utilities|Time|ClearandInvalidateTimerbyHandle (Variables|Default|GetDamageTimerHandle))
  (Utilities|IsValid _fire
    (:Is%20Valid
      (Components|Activation|Deactivate _fire)
      (Components|DestroyComponent _fire))))