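; Scene component that turns its location into an explosion, with sound, particles, damage and knockback, when Explode is called with the exploding actor.
; Explode plays the sound, spawns an attached auto-released emitter and applies full radial damage, with Pawn as the damage prevention channel.
; It then adds a RadialForceComponent to that actor and fires an impulse over the same radius.
; Cleanup code for both spawned components is disconnected, so EndPlay does nothing.
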(event Custom|Explode
  (params (ExplodingActor :type Actor%20Object%20Reference))
  ;[1 1 1] Explode - play explosion sound, apply radial damage, apply radial impulse
  (Variables|Default|SetExplodingActor ExplodingActor)
  (|PlayExplosionSound)
  (|SpawnExplosion)
  (Game|Damage|ApplyRadialDamage)
  (|ApplyRadialForce))

(event EventEndPlay
  (params (EndPlayReason :type EEndPlayReason%20Enum :default "Destroyed"))
  ;[1 1 1] Destroy spawned particle emitter
)