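; Actor component that dissolves a mesh by animating a material parameter over time.
; On BeginPlay it adds a Timeline component to its owner at runtime, binding a float curve and an end-of-timeline event.
; Dissolve swaps slot 0 of the target mesh to a dynamic instance of the dissolve material and plays the timeline.
; The curve drives the DissolveAmount parameter, and completion fires the OnDissolveFinished dispatcher.
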(event Custom|Dissolve
  (bind _meshtodissolve (Variables|Default|GetMeshToDissolve)
    (:then
      (Rendering|Material|SetMaterial _meshtodissolve 0 (Variables|Default|GetMaterial))
      (bind _returnvalue (Rendering|Material|CreateDynamicMaterialInstance (Variables|Default|GetMeshToDissolve) 0 (Variables|Default|GetMaterial) "None" :!class /Script/Engine.PrimitiveComponent))
      (Variables|Default|SetDynamicMaterial _returnvalue)
      (Audio|Components|Audio|Play (Variables|Default|GetTimeline)))
    (:else)))

(event Custom|UpdateDissolveState
  (params (Output :type Float%20%28single-precision%29))
  (Rendering|Material|SetScalarParameterValue (Variables|Default|GetDynamicMaterial) "DissolveAmount" Output :!class /Script/Engine.MaterialInstanceDynamic))

(event Custom|TimelienFinished
  (Default|CallOnDissolveFinished))

(event EventBeginPlay
  (bind _returnvalue (Game|AddComponentbyClass (Components|GetOwner) "/Script/Engine.TimelineComponent"))
  (bind _output_get (Variables|Default|SetTimeline _returnvalue))
  (Class|TimelineComponent|AddInterpFloat _output_get "/Game/NightmareRealm/Components/Dissolve/C_DissolveTimeline.C_DissolveTimeline" (EventDispatchers|CreateEvent :!event Custom|UpdateDissolveState) "None" "None")
  (Audio|AddEvent (Variables|Default|GetTimeline) (Components|Timeline|GetTimelineLength (Variables|Default|GetTimeline)) (EventDispatchers|CreateEvent :!event Custom|TimelienFinished)))