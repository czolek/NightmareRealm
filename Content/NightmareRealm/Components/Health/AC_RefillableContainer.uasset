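; Refillable container component that tracks a fill level up to a max capacity, with an optional world-space fill bar.
; Increase and decrease events adjust the unclamped level and broadcast change events, plus filled or emptied events at the limits.
; BeginPlay creates the WB_FillLevelBar widget and Tick yaws it toward the player camera.
; Replenish sets the level straight to max without broadcasting.
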(event Custom|DecreaseFillLevel
  (params (ByAmount :type Float%20%28double-precision%29))
  ;[1 1 1] Reduce fill level value and, if below or equal zero, send OnEmptied event
  (if (CallFunction|IsNotEmpty)
    (bind _output_get (Variables|Internals|SetFillLevel (- (Variables|Internals|GetFillLevel) ByAmount)))
    (Default|CallOnFillLevelDecreased _output_get)
    (if (<= (Variables|Internals|GetFillLevel) 0.0)
      (Default|CallOnEmptied))))

(event Custom|IncreaseFillLevel
  (params (ByAmount :type Float%20%28double-precision%29))
  ;[1 1 1] Increase fill level, if equal or above max capacity, send OnFilled event
  (if (CallFunction|IsNotFull)
    (bind _output_get (Variables|Internals|SetFillLevel (+ (Variables|Internals|GetFillLevel) ByAmount)))
    (Default|CallOnFillLevelIncreased _output_get)
    (if (>= (Variables|Internals|GetFillLevel) (Variables|Editable|GetMaxCapacity))
      (Default|CallOnFilled))))

(event EventBeginPlay
  ;[1 1 1] Setup Fillbar indicator widget
  (Variables|Internals|SetFillLevel (Variables|Editable|GetInitialFillLevel))
  (if (Variables|Editable|GetHasFillLevelBar)
    (Collision|SetCollisionEnabled "NoCollision")
    (Class|WidgetComponent|SetWidgetSpace "World")
    (Collision|SetCollisionEnabled "QueryAndPhysics")
    (bind _returnvalue (Game|ConstructObjectfromClass "/Game/NightmareRealm/Components/Health/WB_FillLevelBar.WB_FillLevelBar_C" (Variables|Editable|GetInitialFillLevel) (Variables|Editable|GetMaxCapacity) self (Variables|Editable|GetFillLevelBarSize)))
    (bind _output_get (Variables|Internals|SetFillLevelWidget _returnvalue))
    (UserInterface|SetWidget _output_get)))

(event EventTick
  (params (DeltaSeconds :type Float%20%28single-precision%29))
  ;[1 1 1] Rotate fill level bar towards camera
  (if (Variables|Editable|GetHasFillLevelBar)
    (Transformation|SetWorldRotation (Math|Rotator|MakeRotator 0.0 0.0 (.yaw (Math|Rotator|FindLookatRotation (Transformation|GetWorldLocation) (Transformation|GetWorldLocation (Variables|/Script/Engine.PlayerCameraManager|GetTransformComponent (Game|GetPlayerCameraManager 0)))))) false false)))

(fn GetCurrentFillLevel
  (return (Variables|Internals|GetFillLevel)))

(fn IsNotEmpty
  (return (>= (Variables|Internals|GetFillLevel) 0.0)))

(fn IsNotFull
  (return (not (>= (Variables|Internals|GetFillLevel) (Variables|Editable|GetMaxCapacity)))))

(fn Replenish
  (Variables|Internals|SetFillLevel (Variables|Editable|GetMaxCapacity)))