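; Swing trail component that shows a Niagara ribbon-style sword trail during weapon swings.
; On BeginPlay it spawns an inactive NS_SwingTrail attached to itself, centered between the begin and end trail locations, aligned to that segment, with width set to its length.
; SpawnTrail sets the trail lifetime from the given duration and activates the effect, while DestroyTrail deactivates it.
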(event Custom|SpawnTrail
  (params (SpawnDuration :type Float%20%28double-precision%29))
  (bind _swordtrailparticle (Variables|Default|GetSwordTrailParticle)
    (:then
      (Effects|Components|ParticleSystem|SetFloatParameter _swordtrailparticle "TrailLifetime" SpawnDuration)
      (Components|Activation|SetActive _swordtrailparticle true false))
    (:else)))

(event Custom|DestroyTrail
  (bind _swordtrailparticle (Variables|Default|GetSwordTrailParticle)
    (:then
      (Components|Activation|SetActive _swordtrailparticle false false))
    (:else)))

(event EventBeginPlay
  (bind _begintraillocation (Variables|Default|GetBeginTrailLocation))
  (bind _endtraillocation (Variables|Default|GetEndTrailLocation))
  (bind _returnvalue (- _begintraillocation _endtraillocation))
  (bind _returnvalue_2 (Niagara|SpawnSystemAttached "/Game/NightmareRealm/Components/SwingTrail/NS_SwingTrail.NS_SwingTrail" self "" (/ (+ _begintraillocation _endtraillocation) 2.0) (Math|Rotator|MakeRotfromZ _returnvalue) "KeepWorldPosition" false false "None" false))
  (bind _output_get (Variables|Default|SetSwordTrailParticle _returnvalue_2))
  (Effects|Components|ParticleSystem|SetFloatParameter _output_get "TrailWidth" (Math|Vector|VectorLength _returnvalue)))