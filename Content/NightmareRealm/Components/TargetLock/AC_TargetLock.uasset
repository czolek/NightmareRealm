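; AC_TargetLock is a static mesh component that displays a target lock indicator.
; On BeginPlay it configures itself as a small, collision-free plane with the trace indicator material, placed at a configurable relative position.
; Each tick it billboards toward the player camera on yaw only, zeroing world pitch and roll and adding a half-turn to the look-at yaw.
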(event EventTick
  (params (DeltaSeconds :type Float%20%28single-precision%29))
  (Transformation|SetWorldRotation (Math|Rotator|MakeRotator 0.0 0.0 (+ (.yaw (Math|Rotator|FindLookatRotation (Transformation|GetWorldLocation) (Transformation|GetWorldLocation (Variables|/Script/Engine.PlayerCameraManager|GetTransformComponent (Game|GetPlayerCameraManager 0))))) 1.8e+02)) false false))

(event EventBeginPlay
  (Components|StaticMesh|SetStaticMesh "/Game/NightmareRealm/Components/TargetLock/SM_TargetPlane.SM_TargetPlane")
  (Collision|SetCollisionEnabled "NoCollision")
  (Rendering|Material|SetMaterial 0 "/Game/NightmareRealm/Components/TargetLock/MI_TraceIndicator.MI_TraceIndicator")
  (Transformation|SetRelativeLocation (Variables|Default|GetTargetLockRelativePosition) false false)
  (Transformation|SetRelativeRotation "0.000000,180.000000,0.000000" false false)
  (Transformation|SetRelativeScale3D "0.150000,0.150000,0.150000"))