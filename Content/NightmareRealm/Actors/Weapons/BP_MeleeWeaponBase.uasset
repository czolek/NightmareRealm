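; Base melee weapon actor that detects hits with capsule overlaps instead of active sphere traces.
; EnableHitTrace and DisableHitTrace toggle capsule collision and reset a DoOnce, limiting each window to one valid hit.
; Overlaps skip itself, its parent actor, ignore-tagged and undamageable actors, then play a sound and call ApplyDamageTo.
; BeginPlay adds an AC_SwingTrail component; damage, hit sound and trail location functions are empty stubs.
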(event OnComponentBeginOverlap(Capsule)
  (params (OverlappedComponent :type Primitive%20Component%20Object%20Reference) (OtherActor :type Actor%20Object%20Reference) (OtherComp :type Primitive%20Component%20Object%20Reference) (OtherBodyIndex :type Integer) (bFromSweep :type Boolean) (SweepResult :type Hit%20Result%20Structure%20%28by%20ref%29))
  ;[1 1 1] Trace detection by capsule ovelap - more event driven than active sphere trace
  (Utilities|IsValid OtherActor
    (:Is%20Valid
      (if (Math|Boolean|ANDBoolean (!= OtherActor (Actor|GetParentActor)) (!= OtherActor self) (not (Utilities|Array|ContainsItem (Variables|/Script/Engine.Actor|GetTags OtherActor) (Variables|WeaponSetup|GetTagOfActorsToIgnore))) (Variables|/Script/Engine.Actor|GetbCanBeDamaged OtherActor))
        (Utilities|FlowControl|DoOnce false
          (:Completed
            (Utilities|FlowControl|Sequence
              (:then_0
                (bind _sound (Abstract|GetHitSound))
                (Audio|PlaySoundatLocation _sound (Transformation|GetActorLocation) "0, 0, 0" 1.0 1.0 0.0 0 0 0 0))
              (:then_1
                (Abstract|ApplyDamageto OtherActor)))))))))

(event EventBeginPlay
  ;[1 1 1] Initial setup - swing trail
  (bind _locations (Abstract|GetSwingTrailLocations))
  (bind _returnvalue (Game|AddComponentbyClass :Class "/Game/NightmareRealm/Components/SwingTrail/AC_SwingTrail.AC_SwingTrail_C" :BeginTrailLocation (.BeginLocation (Utilities|Struct|BreakS_BeginEndLocation _locations)) :EndTrailLocation (.EndLocation (Utilities|Struct|BreakS_BeginEndLocation _locations))))
  (Components|Activation|Activate _returnvalue false))

(event EventEnableHitTrace
  (bind _capsule (Variables|Default|GetCapsule))
  ;[1 1 1] Enable capsule collision
  (Collision|SetCollisionEnabled _capsule "QueryOnly")
  (Collision|SetCollisionResponsetoChannel _capsule "ECC_Pawn" "ECR_Overlap")
  ;[1 1 1] Trace detection by capsule ovelap - more event driven than active sphere trace
  (Utilities|FlowControl|DoOnce false) ; enters at Reset
)

(event EventDisableHitTrace
  ;[1 1 1] Disbale capsule collision
  (Collision|SetCollisionEnabled (Variables|Default|GetCapsule) "NoCollision")
  ;[1 1 1] Trace detection by capsule ovelap - more event driven than active sphere trace
  (Utilities|FlowControl|DoOnce false) ; enters at Reset
)

(fn ConstructionScript)

(fn ApplyDamageto
  (params (Actor :type Actor%20Object%20Reference)))

(fn GetHitSound
  (return 0))

(fn GetSwingTrailLocations
  (return ""))