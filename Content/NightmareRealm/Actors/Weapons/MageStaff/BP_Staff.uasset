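; BP_Staff is the mage staff weapon actor, dealing damage and supplying its hit sound and swing trail.
; Its actor-hit event applies base damage from the MageStaff row of DT_Weapons and plays the hit sound at the impact.
; ApplyDamageTo instead takes damage from the game instance's magic staff skill stats.
; Getters return the TrailTop and TrailBottom mesh socket locations and the staff hit cue.
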(event Custom|OnActorHitEvent
  (params (ActorHit :type Hit%20Result%20Structure))
  (bind (_bblockinghit _binitialoverlap _time _distance _location _impactpoint _normal _impactnormal _physmat _hitactor) (Collision|BreakHitResult ActorHit))
  (bind _returnvalue (Utilities|GetDataTableRow "/Game/NightmareRealm/DataTables/DT_Weapons.DT_Weapons" "MageStaff")
    (:then
      (Game|Damage|ApplyDamage _hitactor (.BaseDamage (Utilities|Struct|BreakS_WeaponStats _returnvalue)) (Game|GetPlayerController 0) self)
      (Audio|PlaySoundatLocation "/Game/NightmareRealm/Actors/Weapons/MageStaff/Sounds/SW_StaffHit_Cue.SW_StaffHit_Cue" _location "0, 0, 0" 1.0 1.0 0.0 0 0 0 0))))

(event EventBeginPlay
  (|CallParentFunction))

(fn ConstructionScript)

(fn GetSwingTrailLocations
  (return (Utilities|Struct|MakeS_BeginEndLocation (Transformation|GetSocketLocation (Variables|Default|GetWeaponMesh) "TrailTop") (Transformation|GetSocketLocation (Variables|Default|GetWeaponMesh) "TrailBottom"))))

(fn GetHitSound
  (return "/Game/NightmareRealm/Actors/Weapons/MageStaff/Sounds/SW_StaffHit_Cue.SW_StaffHit_Cue"))

(fn ApplyDamageto
  (params (Actor :type Actor%20Object%20Reference))
  (bind _damage (Class|BPISkillSupplier|GetMagicStaffSkillStats(Message) (Game|GetGameInstance)))
  (Game|Damage|ApplyDamage Actor _damage 0 self))