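; BP_Sword is a sword weapon Blueprint that supplies sword-specific sound, trail and damage behavior on top of its parent class.
; It returns the sword hit cue and reports swing trail endpoints from the TrailTop and TrailBottom sockets on the weapon mesh.
; Damage reads BaseDamage from the LightSword row of DT_Weapons and applies it to the given actor with the sword as causer.
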(event EventBeginPlay
  (|CallParentFunction))

(fn ConstructionScript)

(fn GetHitSound
  (return "/Game/NightmareRealm/Actors/Weapons/Sword/Sounds/SW_SwordHit_Cue.SW_SwordHit_Cue"))

(fn GetSwingTrailLocations
  (return (Utilities|Struct|MakeS_BeginEndLocation (Transformation|GetSocketLocation (Variables|Default|GetWeaponMesh) "TrailTop") (Transformation|GetSocketLocation (Variables|Default|GetWeaponMesh) "TrailBottom"))))

(fn ApplyDamageto
  (params (Actor :type Actor%20Object%20Reference))
  (bind _returnvalue (Utilities|GetDataTableRow "/Game/NightmareRealm/DataTables/DT_Weapons.DT_Weapons" "LightSword")
    (:then
      (Game|Damage|ApplyDamage Actor (.BaseDamage (Utilities|Struct|BreakS_WeaponStats _returnvalue)) 0 self))))