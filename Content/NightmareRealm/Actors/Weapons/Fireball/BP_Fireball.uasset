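; BP_Fireball is a projectile that, once hurled, flies toward an optional homing target or along its owner's forward direction until its lifetime expires.
; On overlap with a damageable actor lacking the ignore tag, it applies damage, plays a hit sound and destroys itself.
; Optional explosive and incendiary flags add components at runtime: AC_Explosion on itself at BeginPlay, AC_Fire on the victim at impact, both sparing tagged actors.
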(event OnComponentBeginOverlap(Collision)
  (params (OverlappedComponent :type Primitive%20Component%20Object%20Reference) (OtherActor :type Actor%20Object%20Reference) (OtherComp :type Primitive%20Component%20Object%20Reference) (OtherBodyIndex :type Integer) (bFromSweep :type Boolean) (SweepResult :type Hit%20Result%20Structure%20%28by%20ref%29))
  ;[1 1 1] Apply damage on hit
  (if (and (not (Utilities|Array|ContainsItem (Variables|/Script/Engine.Actor|GetTags OtherActor) (Variables|WeaponSetup|GetTagsOfActorsToIgnore))) (Variables|/Script/Engine.Actor|GetbCanBeDamaged OtherActor))
    (Utilities|FlowControl|Sequence
      (:then_0
        (Game|Damage|ApplyDamage OtherActor (Variables|WeaponSetup|GetBase%20Damage) 0 self)
        (Audio|PlaySoundatLocation "/Game/NightmareRealm/Actors/Weapons/Fireball/Sound/SW_FireballHit_Cue.SW_FireballHit_Cue" (Transformation|GetActorLocation) "0, 0, 0" 1.0 1.0 0.0 0 0 0 0))
      (:then_1
        (bind _explosioncomponent (Variables|Default|GetExplosionComponent)
          (:then
            (Default|Explode _explosioncomponent self)
            (Development|PrintString "Exploded"))
          (:else)))
      (:then_2
        (if (Variables|WeaponSetup|GetIsIncendiary)
          (bind _returnvalue (Game|AddComponentbyClass :self OtherActor :Class "/Game/NightmareRealm/Components/Fire/AC_Fire.AC_Fire_C" :FireDamagePerTick (Variables|WeaponSetup|GetFire%20Damage%20Per%20Tick) :FireRadius (Variables|WeaponSetup|GetFire%20Radius) :FireTimerTick (Variables|WeaponSetup|GetFire%20Timer%20Tick) :Ignore%20Actors (CallFunction|GetActorstoIgnore)))
          (Default|StartFire _returnvalue)))
      (:then_3
        (Actor|DestroyActor)))))

(event Custom|Hurl
  (bind _projectilemovement (Variables|Default|GetProjectileMovement))
  (bind _homingtarget (Variables|WeaponSetup|GetHomingTarget))
  ;[1 1 1] Hurl the fireball
  (Utilities|Time|SetTimerbyEvent (delegate Custom|FireballTTLExpired) (Variables|WeaponSetup|GetFirebalTTL))
  (Components|Activation|Activate (Variables|Default|GetProjectileMovement) true)
  (Utilities|IsValid _homingtarget
    (:Is%20Valid
      (Variables|/Script/Engine.ProjectileMovementComponent|SetHomingTargetComponent (Variables|Default|GetProjectileMovement) (Variables|/Script/Engine.Character|GetCapsuleComponent _homingtarget))
      (bind _output_get (Variables|/Script/Engine.ProjectileMovementComponent|SetInitialSpeed _projectilemovement (Variables|WeaponSetup|GetSpeed)))
      (Variables|/Script/Engine.ProjectileMovementComponent|SetMaxSpeed _projectilemovement _output_get))
    (:Is%20Not%20Valid
      (Variables|/Script/Engine.MovementComponent|SetVelocity (Variables|Default|GetProjectileMovement) (* (Class|KismetMathLibrary|VectorNormal2D (Transformation|GetActorForwardVector (Components|GetOwner)) 0.0001) (Math|Float|MakeLiteralFloat (Variables|WeaponSetup|GetSpeed)))))))

(event Custom|FireballTTLExpired
  ;[1 1 1] Hurl the fireball
  (Actor|DestroyActor))

(event EventBeginPlay
  ;[1 1 1] Setup explosive component if enabled
  (if (Variables|WeaponSetup|GetIsExplsive)
    (bind _returnvalue (Game|AddComponentbyClass :Class "/Game/NightmareRealm/Components/Explosion/AC_Explosion.AC_Explosion_C" :ExplosionDamage (Variables|WeaponSetup|GetExplosion%20Damage) :ExplosionRadius (Variables|WeaponSetup|GetExplosion%20Radius) :ExplosionImpulseStrength (Variables|Internals|GetExplosion%20Impulse%20Strength) :Ignore%20Actors (CallFunction|GetActorstoIgnore)))
    (Variables|Default|SetExplosionComponent _returnvalue)
    (Development|PrintString "Explosive damage enabled")))

(fn ConstructionScript)

(fn GetActorstoIgnore
  (bind _outactors (Actor|GetAllActorswithTag (Variables|WeaponSetup|GetTagsOfActorsToIgnore)))
  (return _outactors))