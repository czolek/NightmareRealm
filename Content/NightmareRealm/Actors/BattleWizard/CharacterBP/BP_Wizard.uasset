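; Battle wizard character with staff attacks, a fireball spell and target lock-on.
; Lock-on picks a targettable character from a camera-forward sphere sweep, turns the mesh toward it each tick and releases it beyond range.
; Skill stats from the GameInstance drive attack montages and rate-limited fireball spawns that home on the locked target.
; ABP_Wizard handles hit, death, resurrection and celebration animations, with collision restored once resurrection finishes.
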(event Custom|BindOnTraceTargetDeath
  ;[1 1 1] Bind to OnDeathEvent of TargettableCharacter
  (bind _tracedtarget (Variables|CameraLock|GetTracedTarget)
    (:then
      (EventDispatchers|BindEventtoOnDeath _tracedtarget (EventDispatchers|CreateEvent :!event DisableTrace)))
    (:else)))

(event Custom|Celebrate
  ;[1 1 1] Celebrate finishing the level
  (Variables|/Game/NightmareRealm/Actors/BattleWizard/CharacterBP/ABP_Wizard.ABP_Wizard_C|SetIsCelebrating (Variables|Internals|GetAnimationInstance) true))

(event Custom|PlaySpellcastAnimation
  (bind _fireballstats (Variables|Internals|GetFireballStats))
  (bind (_isenabled _isexplosive _isincendiary _attackspeed _basedamage _explosiondamage _explosionradius _burningdamage _burningradius _burningtickfrequency) (Utilities|Struct|BreakS_FireballSkillStats _fireballstats))
  ;[1 1 1] In the future there might be more than one spell - here we should select the active one
  (if _isenabled
    (Default|PlaySpellCastAnimation (Variables|Internals|GetAnimationInstance) _attackspeed)))

(event Custom|Event_OnResurrectionAnimationFinished
  ;[1 1 1] Ressurection
  (Collision|SetCollisionEnabled (Variables|Collision|GetCapsuleComponent) "QueryAndPhysics")
  (Default|CallOnResurrected))

(event Custom|StaffAttack
  ;[1 1 1] Run Attack animation when attack action triggered
  (bind (_damage _attackspeed _montage) (Class|BPISkillSupplier|GetMagicStaffSkillStats(Message) (Game|GetGameInstance)))
  (Default|PlayStaffAttackAnimation (Variables|Internals|GetAnimationInstance) _attackspeed _montage))

(event Custom|ToggleCameraLock
  ;[1 1 1] Enable/disable facing enemy by character
  (bind _tracedtarget (Variables|CameraLock|GetTracedTarget)
    (:then
      (CallFunction|DisableTrace _tracedtarget))
    (:else
      (CallFunction|EnableTraceonNearestTarget)
      (CallFunction|BindonTraceTargetDeath))))

(event Custom|Resurrect
  ;[1 1 1] Ressurection
  (Variables|/Game/NightmareRealm/Actors/BattleWizard/CharacterBP/ABP_Wizard.ABP_Wizard_C|SetIsDead (Variables|Internals|GetAnimationInstance) false))

(event Custom|Died
  ;[1 1 1] Death
  (Variables|/Game/NightmareRealm/Actors/BattleWizard/CharacterBP/ABP_Wizard.ABP_Wizard_C|SetIsDead (Variables|Internals|GetAnimationInstance) true)
  (Collision|SetCollisionEnabled (Variables|Collision|GetCapsuleComponent) "NoCollision"))

(event EventTick
  (params (DeltaSeconds :type Float%20%28single-precision%29))
  ;[1 1 1] Turn character towards target, disable tracking when out of range
  (Utilities|FlowControl|Sequence
    (:then_0
      (CallFunction|FaceCharacterTowardsTarget))
    (:then_1
      (CallFunction|DisableTraceifOutOfRange))))

(event Game|Damage|EventAnyDamage
  (params (Damage :type Float%20%28single-precision%29) (DamageType :type Damage%20Type%20Object%20Reference) (InstigatedBy :type Controller%20Object%20Reference) (DamageCauser :type Actor%20Object%20Reference))
  ;[1 1 1] Damage received
  (Default|CallOnDamageReceived Damage)
  (Default|PlayHitREactionAnimation (Variables|Internals|GetAnimationInstance)))

(event EventCastActiveSpell
  (bind _fireballstats (Variables|Internals|GetFireballStats))
  (bind (_isenabled _isexplosive _isincendiary _attackspeed _basedamage _explosiondamage _explosionradius _burningdamage _burningradius _burningtickfrequency) (Utilities|Struct|BreakS_FireballSkillStats _fireballstats))
  ;[1 1 1] In the future there might be more than one spell - here we should select the active one
  (Utilities|HurlFireball _attackspeed _isexplosive _isincendiary _basedamage _explosiondamage _burningdamage _explosionradius _burningradius _burningtickfrequency))

(event EventBeginPlay
  ;[1 1 1] Setup AnimInstance Reference
  (|CallParentFunction)
  (bind _returnvalue (Utilities|GetDataTableRow "/Game/NightmareRealm/DataTables/DT_Weapons.DT_Weapons" "MageStaff")
    (:then
      (Variables|Internals|SetMagicStaffStats _returnvalue)
      (bind _asabp_wizard (Utilities|Casting|CastToABP_Wizard (Components|SkeletalMesh|GetAnimInstance (Variables|Character|GetMesh))))
      (bind _output_get (Variables|Internals|SetAnimationInstance _asabp_wizard))
      (EventDispatchers|BindEventtoOnResurrectionAnimationFinished _output_get (EventDispatchers|CreateEvent :!event Custom|Event_OnResurrectionAnimationFinished))
      (bind _stats (Class|BPISkillSupplier|GetFireballSkillStats(Message) (Game|GetGameInstance)))
      (Variables|Internals|SetFireballStats _stats))))

(fn ConstructionScript)

(fn FaceCharacterTowardsTarget
  (bind _tracedtarget (Variables|CameraLock|GetTracedTarget)
    (:then
      (LocalVariables|SetTracedActorLocation (Transformation|GetActorLocation _tracedtarget))
      (Transformation|SetWorldRotation (Variables|Character|GetMesh) (|GetAdjustedLookAtRotation (Transformation|GetActorLocation) (LocalVariables|GetTracedActorLocation)) false false))
    (:else)))

(fn EnableTraceonNearestTarget
  (bind _detectedpawns (|TraceForTargets))
  (bind _closesttarget__nullable_ (CallFunction|FindClosestTarget _detectedpawns))
  (Utilities|IsValid _closesttarget__nullable_
    (:Is%20Valid
      (if (!= _closesttarget__nullable_ (Variables|CameraLock|GetTracedTarget))
        (Class|BPITraceable|TraceDisabled(Message) (Variables|CameraLock|GetTracedTarget))
        (bind _asbp_targettable_character (Utilities|Casting|CastToBP_TargettableCharacter _closesttarget__nullable_))
        (bind _output_get (Variables|CameraLock|SetTracedTarget _asbp_targettable_character))
        (Class|BPITraceable|TraceEnabled(Message) _output_get)
        (else
          (Development|PrintString "Same Target"))))
    (:Is%20Not%20Valid
      (Development|PrintString "No pawn detected in vicinity"))))

(fn FindClosestTarget
  (params (Pawns :type Array%20of%20Actor%20Object%20References))
  (if (Utilities|Array|IsValidIndex Pawns)
    (bind _output_get (LocalVariables|SetClosestPawn (Utilities|Array|Get(acopy) Pawns)))
    (LocalVariables|SetCharacterLocation (Transformation|GetWorldLocation (Variables|Character|GetMesh)))
    (LocalVariables|SetClosestDistance (Math|Vector|Distance2D(Vector) (Transformation|GetActorLocation _output_get) (LocalVariables|GetCharacterLocation)))
    (for _array_element Pawns
      (if (< (Math|Vector|Distance2D(Vector) (Transformation|GetActorLocation (LocalVariables|GetClosestPawn)) (LocalVariables|GetCharacterLocation)) (LocalVariables|GetClosestDistance))
        (LocalVariables|SetClosestPawn _array_element)
        (LocalVariables|SetClosestDistance (Math|Vector|Distance2D(Vector) (Transformation|GetActorLocation (LocalVariables|GetClosestPawn)) (LocalVariables|GetCharacterLocation)))))
    (Development|PrintString (Utilities|String|Append "Closest pawn: " (Utilities|GetDisplayName (LocalVariables|GetClosestPawn))))
    (return (LocalVariables|GetClosestPawn))
    (else
      (Development|PrintString "No pawn detected")
      (return 0))))

(fn DisableTrace
  (params (EnemyRef :type BP%20Enemy%20Character%20Base%20Object%20Reference))
  (Class|BPITraceable|TraceDisabled(Message) EnemyRef)
  (Variables|CameraLock|SetTracedTarget 0)
  (Transformation|SetRelativeRotation (Variables|Character|GetMesh) "0.000000,-90.000000,0.000000" false false)
  (Development|PrintString "Trace disabled"))

(fn DisableTraceifOutOfRange
  (bind _tracedtarget (Variables|CameraLock|GetTracedTarget)
    (:then
      (if (> (Math|Vector|Distance2D(Vector) (Transformation|GetActorLocation) (Transformation|GetActorLocation _tracedtarget)) (Variables|CameraLock|GetTargetTraceDistance))
        (Class|BPITraceable|TraceDisabled(Message) _tracedtarget)
        (Variables|CameraLock|SetTracedTarget 0)
        (Transformation|SetRelativeRotation (Variables|Character|GetMesh) "0.000000,-90.000000,0.000000" false false)))
    (:else)))