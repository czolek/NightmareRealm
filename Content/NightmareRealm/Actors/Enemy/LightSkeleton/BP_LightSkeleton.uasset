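; BP_LightSkeleton is the light skeleton enemy character, with an attack montage, stat-driven movement speeds and an energy gain value.
; On BeginPlay it reads its DT_Enemies row and creates an AC_RefillableContainer as health, binding to its emptied event.
; Damage drains health and plays a hit reaction.
; Kill notifies the controller, ragdolls the mesh, broadcasts OnDeath, then after a delay dissolves the body through ACDissolve and destroys the actor.
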(event Custom|Dissolve
  (bind _ac_dissolve (Variables|Default|GetAC_Dissolve))
  ;[1 1 1] Dissolve the body and destroy the actor
  (Variables|/Game/NightmareRealm/Components/Dissolve/AC_Dissolve.AC_Dissolve_C|SetMeshToDissolve _ac_dissolve (Variables|Character|GetMesh))
  (EventDispatchers|BindEventtoOnDissolveFinished _ac_dissolve (delegate Custom|DissolveFinished))
  (Default|Dissolve (Variables|Default|GetAC_Dissolve)))

(event Custom|DissolveFinished
  ;[1 1 1] Dissolve the body and destroy the actor
  (Actor|DestroyActor))

(event EventKill
  ;[1 1 1] Enable ragdoll effect on death
  (Audio|PlaySoundatLocation "/Game/NightmareRealm/Actors/Enemy/LightSkeleton/Sounds/SW_Hiss_Cue.SW_Hiss_Cue" (Transformation|GetActorLocation) "0, 0, 0" 1.0 1.0 0.0 0 0 0 0)
  (Class|BPIAiControllerEvents|OnDeathOfControlledPawn(Message) (Pawn|GetController))
  (Physics|SetSimulatePhysics (Variables|Character|GetMesh) true)
  (Collision|SetCollisionEnabled (Variables|Character|GetMesh) "PhysicsOnly")
  (Collision|SetCollisionEnabled (Variables|Default|GetCapsuleComponent) "NoCollision")
  (Utilities|FlowControl|Sequence
    (:then_0
      (bind _healthcomponent (Variables|Default|GetHealthComponent)
        (:then
          (Components|Activation|Deactivate _healthcomponent)
          (Components|DestroyComponent _healthcomponent))
        (:else)))
    (:then_1
      (CallFunction|TraceDisabled)
      (Utilities|FlowControl|Delay (Variables|Default|GetDissolveDelayDuration))
      (CallFunction|Dissolve))
    (:then_2
      (Default|CallOnDeath self))))

(event Game|Damage|EventAnyDamage
  (params (Damage :type Float%20%28single-precision%29) (DamageType :type Damage%20Type%20Object%20Reference) (InstigatedBy :type Controller%20Object%20Reference) (DamageCauser :type Actor%20Object%20Reference))
  ;[1 1 1] React to damage
  (bind _healthcomponent (Variables|Default|GetHealthComponent)
    (:then
      (Default|DecreaseFillLevel _healthcomponent Damage)
      (Animation|Montage|PlayMontage (Variables|Character|GetMesh) "/Game/NightmareRealm/Actors/Enemy/LightSkeleton/Animations/AM_HitReaction.AM_HitReaction"))
    (:else)))

(event EventBeginPlay
  ;[1 1 1] Bind to OnDeath event
  (bind _returnvalue (Utilities|GetDataTableRow "/Game/NightmareRealm/DataTables/DT_Enemies.DT_Enemies" "LightSkeleton")
    (:then
      (bind _output_get (Variables|Default|SetStats _returnvalue))
      (bind _returnvalue_2 (Game|AddComponentbyClass "/Game/NightmareRealm/Components/Health/AC_RefillableContainer.AC_RefillableContainer_C" false (Math|Transform|MakeTransform (Variables|HealthBar|GetHealthBarRelativeLocation) "0, 0, 0" "1.000000,1.000000,1.000000") (.BasicHealth (Utilities|Struct|BreakS_EnemyStats _output_get)) (Variables|HealthBar|GetHasHealthBar) (Variables|HealthBar|GetHealthBarSize) (.BasicHealth (Utilities|Struct|BreakS_EnemyStats _output_get))))
      (bind _output_get_2 (Variables|Default|SetHealthComponent _returnvalue_2))
      (EventDispatchers|BindEventtoOnEmptied _output_get_2 (EventDispatchers|CreateEvent :!event Kill)))))

(event EventSetMovementSpeed
  (params (MovementSpeed :type E_MovementSpeed%20Enum :default "NewEnumerator0"))
  (bind _stats (Variables|Default|GetStats))
  (bind (_basichealth _basewalkingspeed _baserunningspeed) (Utilities|Struct|BreakS_EnemyStats _stats))
  ;[1 1 1] Set movement speed based on bahaviour
  (Variables|/Script/Engine.CharacterMovementComponent|SetMaxWalkSpeed (Variables|Character|GetCharacterMovement) (Utilities|Select :Index MovementSpeed :NewEnumerator0 0.0 :NewEnumerator1 _basewalkingspeed :NewEnumerator2 _baserunningspeed)))

(fn ConstructionScript)

(fn GetEnergyGain
  (return (.EnergyGain (Utilities|Struct|BreakS_EnemyStats (Variables|Default|GetStats)))))

(fn Attack
  (bind _returnvalue (Animation|PlayAnimMontage "/Game/NightmareRealm/Actors/Enemy/LightSkeleton/Animations/AM_Attack.AM_Attack" 1.0 "None"))
  (return _returnvalue))