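; BP_Pylon is a glowing, levitating, rotating pylon that relays damage and either explodes or shuts down.
; Looping timers drive spin and sine-wave levitation instead of Tick, and construction applies the light settings.
; EnergyFull runs timeline-driven implosion and explosion effects with sound, light and scaling.
; Destroyed swaps the idle timers for one that interpolates light, local offset and world height to zero, then clears itself.
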(event Custom|Destroyed
  (|Animateshutdown))

(event Custom|EnergyFull
  (|Explode))

(event EventBeginPlay
  (|Animate))

(event Game|Damage|EventAnyDamage
  (params (Damage :type Float%20%28single-precision%29) (DamageType :type Damage%20Type%20Object%20Reference) (InstigatedBy :type Controller%20Object%20Reference) (DamageCauser :type Actor%20Object%20Reference))
  (Default|CallOnDamageReceived Damage))

(fn ConstructionScript
  (Rendering|Components|Light|SetLightColor (Variables|Default|GetPointLight) (Variables|Editable|GetLightColor) true)
  (Class|LightComponent|SetTemperature (Variables|Default|GetPointLight) (Variables|Editable|GetLightTemperature))
  (Rendering|Components|Light|SetIntensity (Variables|Default|GetPointLight) (Variables|Editable|GetLightIntensity)))

(event Custom|DisablePylon
  (Utilities|FlowControl|Sequence
    (:then_0
      (|Fadeawaythelight))
    (:then_1
      (|Nullifiylocaloffset))
    (:then_2
      (|Falldowntotheground))
    (:then_3
      (|Stopanimationtickonceallabovevaluesaredownto0))))

(event Custom|Rotate
  (Transformation|AddLocalRotation (Variables|Default|GetPylon) (Math|Rotator|MakeRotator 0.0 0.0 (* (Variables|Default|GetRotationTick) (Variables|Editable|GetRotationDegreesPerSecond))) false false))

(event Custom|Levitate
  (Transformation|AddLocalOffset (Variables|Default|GetPylon) (Math|Vector|MakeVector 0.0 0.0 (* (* (Variables|Editable|GetLevitationDistance) (Variables|Default|GetLevitationTick)) (Math|Trig|Sin(Radians) (* (Utilities|Time|GetGameTimeinSeconds) (Variables|Editable|GetLevitationSpeed))))) false false))