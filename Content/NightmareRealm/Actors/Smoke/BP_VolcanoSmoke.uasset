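; BP_VolcanoSmoke is an actor that emits intermittent volcano smoke bursts with a hissing sound.
; From BeginPlay, an endless event loop waits a random pause, activates the geyser smoke effect and hiss audio, then stops both after a random burst duration.
; Two range variables set the minimum and maximum for the pause and burst lengths, randomized each cycle with Delay nodes rather than Tick.
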(event Custom|SmokeBurst
  (bind _smokeburstdurationrandomrange (Variables|Default|GetSmokeBurstDurationRandomRange))
  (bind (_x _y) (Math|Vector2D|BreakVector2D _smokeburstdurationrandomrange))
  (Components|Activation|Activate (Variables|Default|GetN_GeyserSmoke) false)
  (Audio|Components|Audio|Play (Variables|Default|GetSW_Hiss_Cue) 0.0)
  (Utilities|FlowControl|Delay (Math|Random|RandomFloatinRange _x _y))
  (CallFunction|StopSmoke))

(event Custom|EmitSmoke
  (bind _smokeburstpausedurationrandomrange (Variables|Default|GetSmokeBurstPauseDurationRandomRange))
  (bind (_x _y) (Math|Vector2D|BreakVector2D _smokeburstpausedurationrandomrange))
  (Utilities|FlowControl|Delay (Math|Random|RandomFloatinRange _x _y))
  (CallFunction|SmokeBurst))

(event Custom|StopSmoke
  (Components|Activation|Deactivate (Variables|Default|GetN_GeyserSmoke))
  (Audio|Components|Audio|Stop (Variables|Default|GetSW_Hiss_Cue))
  (CallFunction|EmitSmoke))

(event EventBeginPlay
  (CallFunction|EmitSmoke))

(fn ConstructionScript)