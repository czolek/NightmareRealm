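; Enemy spawner actor that spawns enemy characters through a portal effect while IsActive is set.
; SpawnEnemy async-loads the requested class, activates the portal, plays its sound, spawns the pawn, fires OnEnemySpawned, then deactivates the portal after a short delay.
; Pawns spawn at the actor's location facing the Arrow's direction, adjusting for collisions, and get a default controller.
; A test event spawns a Light Skeleton.
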(event Custom|SpawnEnemy
  (params (EnemyClass :type BP%20Enemy%20Character%20Base%20Soft%20Class%20Reference))
  (if (Variables|Default|GetIsActive)
    (bind _class (Utilities|AsyncLoadClassAsset EnemyClass)
      (:Completed
        (bind _asbp_enemy_character_base (Utilities|Casting|CastToBP_EnemyCharacter_BaseClass _class))
        (Utilities|FlowControl|Sequence
          (:then_0
            (CallFunction|ActivatePortal))
          (:then_1
            (CallFunction|PlayPortalSound))
          (:then_2
            (bind _spawnedenemycharacter (CallFunction|SpawnPawn _asbp_enemy_character_base))
            (Default|CallOnEnemySpawned _spawnedenemycharacter)
            (Utilities|FlowControl|Delay 0.5)
            (CallFunction|DeactivatePortal)))))))

(event Custom|TestSpawnLightSkeleton
  (CallFunction|SpawnEnemy "/Game/NightmareRealm/Actors/Enemy/LightSkeleton/BP_LightSkeleton.BP_LightSkeleton_C"))

(fn ConstructionScript)

(fn PlayPortalSound
  (Audio|PlaySoundatLocation (Variables|/Script/Engine.AudioComponent|GetSound (Variables|Default|GetSW_EnterThroughPortal_Cue)) (Transformation|GetActorLocation) "0, 0, 0" 1.0 1.0 0.0 0 0 0 0))

(fn ActivatePortal
  (Components|Activation|Activate (Variables|Default|GetPortal) false))

(fn DeactivatePortal
  (Components|Activation|Deactivate (Variables|Default|GetPortal)))

(fn SpawnPawn
  (params (EnemyCharacter :type BP%20Enemy%20Character%20Base%20Class%20Reference))
  (bind _returnvalue (Game|SpawnActorfromClass EnemyCharacter (Math|Transform|MakeTransform (Transformation|GetActorLocation) (Transformation|GetWorldRotation (Variables|Default|GetArrow))) "AdjustIfPossibleButAlwaysSpawn" "OverrideRootScale" 0 0))
  (Utilities|IsValid _returnvalue
    (:Is%20Valid
      (Pawn|SpawnDefaultController _returnvalue)
      (return _returnvalue))))